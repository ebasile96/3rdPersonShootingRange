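; BP_TargetManager runs a shooting-gallery loop, keeping a target spawned at random points and awarding score for hits.
; On BeginPlay it caches locations of actors tagged "Spot", finds the score manager and player, then spawns a BP_Target at a random cached point.
; Each target's hit event adds points, plays an impact sound at the player, and after a short delay spawns the next target.
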(event Custom|OnHit
  (Variables|/Game/Blueprints/BP_ScoreManager.BP_ScoreManager_C|SetTotalScore (Variables|Default|GetScoreMgr) (+ (Variables|/Game/Blueprints/BP_ScoreManager.BP_ScoreManager_C|GetTotalScore (Variables|Default|GetScoreMgr)) 1e+02))
  (Audio|SpawnSoundatLocation "/Game/Sound/Impact.Impact" (Transformation|GetActorLocation (Variables|Default|GetPlayer)) "0, 0, 0" 1.0 1.0 0.0 0 0)
  (Utilities|FlowControl|Delay 0.5)
  (bind _returnvalue (Game|SpawnActorfromClass "/Game/Blueprints/BP_Target.BP_Target_C" (Math|Conversions|ToTransform(Vector) (Utilities|Array|Get(acopy) (Variables|Default|GetTargetPoints) (Math|Random|RandomInteger (Utilities|Array|Length (Variables|Default|GetTargetPoints))))) "Undefined" 0 0))
  (EventDispatchers|BindEventtoOnTargetHit _returnvalue (delegate Custom|OnHit))
  (Audio|SpawnSoundatLocation "/Game/Sound/tARGETsPAWNsOUND.TargetSpawnSound" (Transformation|GetActorLocation (Variables|Default|GetPlayer)) "0, 0, 0" 1.0 1.0 0.0 0 0))

(event EventBeginPlay
  (Utilities|FlowControl|Sequence
    (:then_0
      (bind _outactors (Actor|GetAllActorswithTag "Spot"))
      (for _array_element _outactors
        (Utilities|Array|Add (Variables|Default|GetTargetPoints) (Transformation|GetActorLocation _array_element))))
    (:then_1
      (bind _returnvalue (Actor|GetActorOfClass "/Game/Blueprints/BP_ScoreManager.BP_ScoreManager_C"))
      (Variables|Default|SetScoreMgr _returnvalue))
    (:then_2
      (bind _returnvalue_2 (Actor|GetActorOfClass "/Game/AnimStarterPack/Ue4ASP_Character.Ue4ASP_Character_C"))
      (Variables|Default|SetPlayer _returnvalue_2))
    (:then_3
      (bind _returnvalue_3 (Game|SpawnActorfromClass "/Game/Blueprints/BP_Target.BP_Target_C" (Math|Conversions|ToTransform(Vector) (Utilities|Array|Get(acopy) (Variables|Default|GetTargetPoints) (Math|Random|RandomInteger (Utilities|Array|Length (Variables|Default|GetTargetPoints))))) "Undefined" 0 0))
      (EventDispatchers|BindEventtoOnTargetHit _returnvalue_3 (delegate Custom|OnHit))
      (Audio|SpawnSoundatLocation "/Game/Sound/tARGETsPAWNsOUND.TargetSpawnSound" (Transformation|GetActorLocation (Variables|Default|GetPlayer)) "0, 0, 0" 1.0 1.0 0.0 0 0))))

(fn ConstructionScript)