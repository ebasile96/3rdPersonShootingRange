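; Game manager Blueprint that runs a timed score round and ends it with a win or lose screen.
; On BeginPlay it caches the BP_ScoreManager, sets game-only input and starts a 60-second one-shot timer, whose remaining time Tick copies into TimeLeft.
; When the timer fires, it compares TotalScore to a fixed threshold, shows the matching widget and switches to UI input with the cursor visible.
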(event Custom|GameOverScreen
  (bind _returnvalue (Game|GetPlayerController 0))
  (bind _returnvalue_2 (Game|GetPlayerController 0))
  (if (>= (Variables|/Game/Blueprints/BP_ScoreManager.BP_ScoreManager_C|GetTotalScore (Variables|Default|GetScoreMgr)) 2.5e+03)
    (bind _returnvalue_3 (UserInterface|CreateWidget "/Game/Blueprints/UI/WinWidget.WinWidget_C"))
    (UserInterface|Viewport|AddtoViewport _returnvalue_3 0)
    (Input|SetInputModeUIOnly _returnvalue_2 0 "DoNotLock")
    (Variables|/Script/Engine.PlayerController|SetbShowMouseCursor _returnvalue_2 true)
    (else
      (bind _returnvalue_4 (UserInterface|CreateWidget "/Game/Blueprints/UI/LoseWidget.LoseWidget_C"))
      (UserInterface|Viewport|AddtoViewport _returnvalue_4 0)
      (Input|SetInputModeUIOnly _returnvalue 0 "DoNotLock")
      (Variables|/Script/Engine.PlayerController|SetbShowMouseCursor _returnvalue true))))

(event EventBeginPlay
  (bind _returnvalue (Game|GetPlayerController 0))
  (Utilities|FlowControl|Sequence
    (:then_0
      (bind _returnvalue_2 (Actor|GetActorOfClass "/Game/Blueprints/BP_ScoreManager.BP_ScoreManager_C"))
      (Variables|Default|SetScoreMgr _returnvalue_2))
    (:then_1
      (Input|SetInputModeGameOnly _returnvalue)
      (Variables|/Script/Engine.PlayerController|SetbShowMouseCursor _returnvalue false))
    (:then_2
      (bind _returnvalue_3 (Utilities|Time|SetTimerbyEvent (delegate Custom|GameOverScreen) 6e+01))
      (Variables|Default|SetTimerValue _returnvalue_3))))

(event EventTick
  (params (DeltaSeconds :type Float%20%28single-precision%29))
  (Variables|Default|SetTimeLeft (Utilities|Time|GetTimerRemainingTimebyHandle (Variables|Default|GetTimerValue))))

(fn ConstructionScript)